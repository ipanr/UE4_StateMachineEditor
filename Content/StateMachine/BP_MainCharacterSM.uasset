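; Data-driven state machine for the main character that picks the current state from a list of detections.
; On BeginPlay it caches each state's accessible transitions from DT_MainCharacterStates into a map.
; Each Tick, when its detection check passes, it filters transitions by required detections and takes the lowest Priority value among multiple candidates.
; A state change reloads the accessible list; debug prints and an empty-detection override remain.
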(event `self.ReceiveBeginPlay`
  (`self.MapStatesAndAccesibleStates`)
  (set `self.globalListOfAccesibleStates` (`.listOfAccesibleStates_3_464E59AE46788B5EE38FAC822782BB6E` (break `/Game/StateMachine/STR_ListOfAccesibleStates` (`BlueprintMapLibrary.Map_Find` (`self.mapStateToAccesibleStates`) "NewEnumerator0")))))

(event `self.ReceiveTick`
  (params (DeltaSeconds :type "Float (single-precision)"))
  (`self.State Machine Logic` (`self.Detections`))
  (`KismetSystemLibrary.PrintString` (`|GetEnumeratorNameAsString` (`self.globalInitialState`))))

(fn `CheckDifferentDetections`
  (params (currentState :type "/Game/StateMachine/UI_StateMachine/ENUM_States Enum" :default "NewEnumerator0") (oldDetections :type "Array of Name") (newDetections :type "Array of Name"))
  (returns (detectionListChanged :type Boolean))
  (locals (differentDetections :type Boolean))
  (bind _returnvalue (`KismetArrayLibrary.Array_Length` newDetections))
  (`|ExecutionSequence`
    (:`then_0`
      (if (> _returnvalue 0)
        (if (!= (`KismetArrayLibrary.Array_Length` (`local.oldDetections`)) _returnvalue)
          (set `local.differentDetections` true)
          (else
            (for _array_element (`local.newDetections`)
              (if (`KismetArrayLibrary.Array_Contains` (`local.oldDetections`) _array_element)
                (set `local.differentDetections` true)
                (break)))))
        (elif (== currentState 0)
          (set `local.differentDetections` true))))
    (:`then_1`
      (return (`local.differentDetections`)))))

(fn `DEBUG_CheckForNoDetectionAccesibleStates`
  (returns (accessNewState :type Boolean))
  (locals (localAccesNewState :type Boolean))
  (for _array_element (`.listOfAccesibleStates_3_464E59AE46788B5EE38FAC822782BB6E` (break `/Game/StateMachine/STR_ListOfAccesibleStates` (`BlueprintMapLibrary.Map_Find` (`self.mapStateToAccesibleStates`) "NewEnumerator0")))
    (if (== (`KismetArrayLibrary.Array_Length` (`.Detections_13_4112E80D4F25656B6E7CD29881C1B65B` (break `/Game/StateMachine/UI_StateMachine/Models/STR_AccesibleStates` _array_element))) 0)
      (set `local.localAccesNewState` true)
      (break)))
  (return (`local.localAccesNewState`)))

(fn `DefineFinalStateAfterCheckingPriority`
  (params (listOfCandidateStates :type "Array of /Game/StateMachine/UI_StateMachine/Models/STR_AccesibleStates Structure") (initialState :type "/Game/StateMachine/UI_StateMachine/ENUM_States Enum" :default "NewEnumerator0"))
  (returns (finalState :type "/Game/StateMachine/UI_StateMachine/ENUM_States Enum"))
  (locals (localFinalState :type "/Game/StateMachine/UI_StateMachine/ENUM_States Enum") (highestPriority :type Integer :default 255))
  (bind _returnvalue (`KismetArrayLibrary.Array_Length` listOfCandidateStates))
  (`|ExecutionSequence`
    (:`then_0`
      (if (== _returnvalue 0)
        (set `local.localFinalState` (`local.initialState`))
        (elif (== _returnvalue 1)
          (set `local.localFinalState` (`.State_12_E4F303534EA9FE35C08515A7369D55FD` (break `/Game/StateMachine/UI_StateMachine/Models/STR_AccesibleStates` (`|GetArrayItem` (`local.listOfCandidateStates`)))))
          (else
            (for _array_element (`local.listOfCandidateStates`)
              (bind (_state _priority) (break `/Game/StateMachine/UI_StateMachine/Models/STR_AccesibleStates` _array_element))
              (if (< _priority (`local.highestPriority`))
                (set `local.highestPriority` _priority)
                (set `local.localFinalState` _state)))))))
    (:`then_1`
      (return (`local.localFinalState`)))))

(fn `DefineState`
  (params (initialState :type "/Game/StateMachine/UI_StateMachine/ENUM_States Enum" :default "NewEnumerator0") (accesibleStates :type "Array of /Game/StateMachine/UI_StateMachine/Models/STR_AccesibleStates Structure") (previousDetections :type "Array of Name") (newDetections :type "Array of Name"))
  (returns (finalState :type "/Game/StateMachine/UI_StateMachine/ENUM_States Enum") (listOfAnalizedDetections :type "Array of Name"))
  (locals (detectionsToReturn :type "Array of Name") (differentDetectionsExist :type Boolean) (localFinalState :type "/Game/StateMachine/UI_StateMachine/ENUM_States Enum" :default "NewEnumerator0") (localAccesibleStateCandidates :type "Array of /Game/StateMachine/UI_StateMachine/Models/STR_AccesibleStates Structure"))
  (`|ExecutionSequence`
    (:`then_0`
      (bind _detectionlistchanged (`self.CheckDifferentDetections` (`local.initialState`) (`local.previousDetections`) (`local.newDetections`)))
      (bind _output_get (set `local.differentDetectionsExist` _detectionlistchanged))
      (if _output_get
        (set `local.detectionsToReturn` (`local.newDetections`))
        (else
          (set `local.detectionsToReturn` (`local.previousDetections`))))
      (if (`self.DEBUG_allowEmptyAccesibleStates`)
        (bind _accessnewstate (`self.DEBUG_CheckForNoDetectionAccesibleStates`))
        (set `local.differentDetectionsExist` _accessnewstate)
        (`KismetSystemLibrary.PrintString` "DEBUGGING IN STATE MACHINE DEFINE STATE" true true (struct :`G` 1.0 :`B` 0.072171 :`A` 1.0))))
    (:`then_1`
      (if (`local.differentDetectionsExist`)
        (bind _statesthatcanbeaccesed (`self.ListOfStatesThatCanBeAccesed` (`local.accesibleStates`) (`local.newDetections`)))
        (set `local.localAccesibleStateCandidates` _statesthatcanbeaccesed)
        (bind _finalstate (`self.DefineFinalStateAfterCheckingPriority` (`local.localAccesibleStateCandidates`) (`local.initialState`)))
        (set `local.localFinalState` _finalstate)
        (else
          (set `local.localFinalState` (`local.initialState`)))))
    (:`then_2`
      (return (`local.localFinalState`) (`local.detectionsToReturn`)))))

(fn `ListOfStatesThatCanBeAccesed`
  (params (accesibleStates :type "Array of /Game/StateMachine/UI_StateMachine/Models/STR_AccesibleStates Structure") (newDetections :type "Array of Name"))
  (returns (statesThatCanBeAccesed :type "Array of /Game/StateMachine/UI_StateMachine/Models/STR_AccesibleStates Structure"))
  (locals (neccesaryDetectionsToEnterTheState :type "Array of Name") (listOfCandidateAccesibleStates :type "Array of /Game/StateMachine/UI_StateMachine/Models/STR_AccesibleStates Structure") (currentAccesibleState :type "/Game/StateMachine/UI_StateMachine/Models/STR_AccesibleStates Structure") (localIteration :type Integer))
  (bind _returnvalue (`KismetArrayLibrary.Array_Length` (`local.neccesaryDetectionsToEnterTheState`)))
  (`|ExecutionSequence`
    (:`then_0`
      (for _array_element accesibleStates
        (set `local.currentAccesibleState` _array_element)
        (set `local.neccesaryDetectionsToEnterTheState` (`.Detections_13_4112E80D4F25656B6E7CD29881C1B65B` (break `/Game/StateMachine/UI_StateMachine/Models/STR_AccesibleStates` _array_element)))
        (if (== _returnvalue 0)
          (`KismetArrayLibrary.Array_Add` (`local.listOfCandidateAccesibleStates`) (`local.currentAccesibleState`))
          (elif (not (> _returnvalue (`KismetArrayLibrary.Array_Length` (`local.newDetections`))))
            (set `local.localIteration` 0)
            (for _array_element_2 (`local.neccesaryDetectionsToEnterTheState`)
              (if (`KismetArrayLibrary.Array_Contains` (`local.newDetections`) _array_element_2)
                (`/Engine/EditorBlueprintResources/StandardMacros.IncrementInt` (`local.localIteration`))
                (else
                  (break))))
            (if (== (`local.localIteration`) (`KismetArrayLibrary.Array_Length` (`local.neccesaryDetectionsToEnterTheState`)))
              (`KismetArrayLibrary.Array_Add` (`local.listOfCandidateAccesibleStates`) (`local.currentAccesibleState`)))))))
    (:`then_1`
      (return (`local.listOfCandidateAccesibleStates`)))))

(fn `MapStatesAndAccesibleStates`
  (locals (populatableListOfAccesibleStates :type "Array of /Game/StateMachine/UI_StateMachine/Models/STR_AccesibleStates Structure") (localListOfAccesibleStates :type "/Game/StateMachine/STR_ListOfAccesibleStates Structure"))
  (bind _enumvalue (foreach `/Game/StateMachine/UI_StateMachine/ENUM_States` false)
    (:`LoopBody`
      (bind _returnvalue (`|GetDataTableRow` "/Game/StateMachine/UI_StateMachine/DT_MainCharacterStates.DT_MainCharacterStates" (`KismetStringLibrary.Conv_StringToName` (`|GetEnumeratorNameAsString` _enumvalue)))
        (:`then`
          (`KismetArrayLibrary.Array_Clear` (`local.populatableListOfAccesibleStates`))
          (bind (_state _accesiblestates) (break `/Game/StateMachine/UI_StateMachine/Models/STR_State` _returnvalue))
          (for _array_element _accesiblestates
            (`KismetArrayLibrary.Array_Add` (`local.populatableListOfAccesibleStates`) _array_element))
          (bind _output_get (set `local.localListOfAccesibleStates` (make `/Game/StateMachine/STR_ListOfAccesibleStates` (`local.populatableListOfAccesibleStates`))))
          (`BlueprintMapLibrary.Map_Add` (`self.mapStateToAccesibleStates`) _state _output_get))))))

(fn `SetGlobalListOfAccesibleStates`
  (params (currentState :type "/Game/StateMachine/UI_StateMachine/ENUM_States Enum" :default "NewEnumerator0"))
  (returns (accesibleStatesa :type "Array of /Game/StateMachine/UI_StateMachine/Models/STR_AccesibleStates Structure"))
  (locals (localAccesibleStates :type "Array of /Game/StateMachine/UI_StateMachine/Models/STR_AccesibleStates Structure") (toIdleWalkRun :type "Array of /Game/StateMachine/UI_StateMachine/Models/STR_AccesibleStates Structure"))
  (bind (_value _returnvalue) (`BlueprintMapLibrary.Map_Find` (`self.mapStateToAccesibleStates`) "NewEnumerator0"))
  (bind (_value_2 _returnvalue_2) (`BlueprintMapLibrary.Map_Find` (`self.mapStateToAccesibleStates`) currentState))
  (if _returnvalue_2
    (set `local.localAccesibleStates` (`.listOfAccesibleStates_3_464E59AE46788B5EE38FAC822782BB6E` (break `/Game/StateMachine/STR_ListOfAccesibleStates` _value_2)))
    (elif _returnvalue
      (set `local.localAccesibleStates` (`.listOfAccesibleStates_3_464E59AE46788B5EE38FAC822782BB6E` (break `/Game/StateMachine/STR_ListOfAccesibleStates` _value)))
      (else
        (set `local.localAccesibleStates` (`local.toIdleWalkRun`)))))
  (return (`local.localAccesibleStates`)))

(fn `State Machine Logic`
  (params (detections :type "Array of Name"))
  (returns (currentState :type "/Game/StateMachine/UI_StateMachine/ENUM_States Enum") (statesChanged :type Boolean))
  (locals (finalState :type "/Game/StateMachine/UI_StateMachine/ENUM_States Enum") (localStatesChanged :type Boolean) (localListOfAccesibleStates :type "/Game/StateMachine/STR_ListOfAccesibleStates Structure" :default (struct :`listOfAccesibleStates` "(())")) (populatableListOfAccesibleStates :type "Array of /Game/StateMachine/UI_StateMachine/Models/STR_AccesibleStates Structure"))
  (bind (_finalstate _listofanalizeddetections) (`self.DefineState` (`self.globalInitialState`) (`self.globalListOfAccesibleStates`) (`self.globalPreviousDetections`) detections))
  (set `self.globalPreviousDetections` _listofanalizeddetections)
  (set `local.finalState` _finalstate)
  (bind _output_get (set `local.localStatesChanged` (!= (`self.globalInitialState`) (`local.finalState`))))
  (if _output_get
    (set `self.globalInitialState` (`local.finalState`))
    (`KismetArrayLibrary.Array_Clear` (`self.globalListOfAccesibleStates`))
    (bind _accesiblestatesa (`self.SetGlobalListOfAccesibleStates` (`self.globalInitialState`)))
    (set `self.globalListOfAccesibleStates` _accesiblestatesa))
  (return (`local.finalState`) (`local.localStatesChanged`)))